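; A ladder actor that lets the first-person character climb while inside its trigger box.
; The construction script stacks static mesh pieces downward along local Z, with the count derived from the length of EndOfLadder and PieceSize.
; It also sizes and positions the box to span that length plus an offset.
; Box overlap begin and end call the character's BeginClimbLadder and EndClimbLadder.
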(event OnComponentBeginOverlap(Box)
  (params (OverlappedComponent :type Primitive%20Component%20Object%20Reference) (OtherActor :type Actor%20Object%20Reference) (OtherComp :type Primitive%20Component%20Object%20Reference) (OtherBodyIndex :type Integer) (bFromSweep :type Boolean) (SweepResult :type Hit%20Result%20Structure%20%28by%20ref%29))
  (bind _asfirst_person_character (Utilities|Casting|CastToFirstPersonCharacter OtherActor))
  (Default|BeginClimbLadder _asfirst_person_character "0, 0, 0"))

(event OnComponentEndOverlap(Box)
  (params (OverlappedComponent :type Primitive%20Component%20Object%20Reference) (OtherActor :type Actor%20Object%20Reference) (OtherComp :type Primitive%20Component%20Object%20Reference) (OtherBodyIndex :type Integer))
  (bind _asfirst_person_character (Utilities|Casting|CastToFirstPersonCharacter OtherActor))
  (Default|EndClimbLadder _asfirst_person_character))

(fn ConstructionScript
  (bind _box (Variables|Default|GetBox))
  (bind _endofladder (Variables|Default|GetEndOfLadder))
  (bind _offset (Variables|Default|GetOffset))
  (bind _returnvalue (Math|Vector|VectorLength _endofladder))
  (bind _returnvalue_2 (+ _returnvalue _offset))
  (bind _returnvalue_3 (/ _returnvalue_2 2.0))
  (for _index (range 0 (.ReturnValue (Math|Float|Division(WholeandRemainder) (Math|Vector|VectorLength (Variables|Default|GetEndOfLadder)) (Variables|Default|GetPieceSize))))
    (AddComponent|AddStaticMeshComponent false (Math|Transform|MakeTransform (Math|Vector|MakeVector 0.0 0.0 (* -1 (* _index (Variables|Default|GetPieceSize)))) "0, 0, 0" "1,1,1")))
  (Components|Box|SetBoxExtent _box (Math|Vector|MakeVector 32.0 6e+01 _returnvalue_3) true)
  (Transformation|SetRelativeLocation _box (Math|Vector|MakeVector 0.0 4e+01 (+ (* -1 _returnvalue_3) (Variables|Default|GetOffset))) false false))